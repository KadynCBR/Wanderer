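; BP_OverworldInteractionActor is an overworld trigger that lets the player interact to enter the shop level.
; Its box overlap registers the actor as the BP_OverworldCharacter's interactable and clears that reference when the overlap ends.
; OnInteract fades the camera and audio out, holds the fade, then opens the Shop level after a short delay.
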(event `self.ReceiveActorBeginOverlap`
  (params (OtherActor :type "Actor Object Reference")))

(event `self.Box.OnComponentBeginOverlap`
  (params (OverlappedComponent :type "PrimitiveComponent Object Reference") (OtherActor :type "Actor Object Reference") (OtherComp :type "PrimitiveComponent Object Reference") (OtherBodyIndex :type Integer) (bFromSweep :type Boolean) (SweepResult :type "HitResult Structure (by ref)"))
  (bind _asbp_overworld_character (cast `/Game/Blueprints/Character/BP_OverworldCharacter` OtherActor))
  (`/Game/Blueprints/Character/BP_OverworldCharacter.SetInteractable` _asbp_overworld_character self))

(event `self.Box.OnComponentEndOverlap`
  (params (OverlappedComponent :type "PrimitiveComponent Object Reference") (OtherActor :type "Actor Object Reference") (OtherComp :type "PrimitiveComponent Object Reference") (OtherBodyIndex :type Integer))
  (bind _asbp_overworld_character (cast `/Game/Blueprints/Character/BP_OverworldCharacter` OtherActor))
  (`/Game/Blueprints/Character/BP_OverworldCharacter.SetInteractable` _asbp_overworld_character null))

(event `OnInteract`
  (`PlayerCameraManager.StartCameraFade` :`self` (`GameplayStatics.GetPlayerCameraManager` 0) :`FromAlpha` 0.0 :`ToAlpha` 1.0 :`Duration` 1.0 :`bShouldFadeAudio` true :`bHoldWhenFinished` true)
  (`KismetSystemLibrary.Delay` 1.5)
  (`GameplayStatics.OpenLevelBySoftObjectPtr` "/Game/Maps/Shop.Shop"))

(fn `UserConstructionScript`)