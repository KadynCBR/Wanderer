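; Player-controlled overworld character with flipbook sprite animation, walking movement and interaction with objects.
; BeginPlay adds the Enhanced Input mapping context, and move input drives normalized movement with inverted Y.
; SetFlipBook picks one of four directional walk flipbooks, giving vertical input priority and using walk-forward when input is zero.
; SetInteractable stores the current target and toggles an indicator with sound, while the Interact action calls OnInteract on it.
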(event `self.ReceiveBeginPlay`
  (bind _asplayer_controller (cast `PlayerController` (`self.GetController`)))
  (`EnhancedInputSubsystemInterface.AddMappingContext` (pcsubsystem `EnhancedInputLocalPlayerSubsystem` _asplayer_controller) "/Game/Input/IMC_PlayerInputContext.IMC_PlayerInputContext" 0 (struct)))

(event `EnhancedInput|/Game/Input/Actions/IA_MoveAction`
  (params (ActionValue :type "Vector2D Structure") (ElapsedSeconds :type "Float (double-precision)") (TriggeredSeconds :type "Float (double-precision)") (InputAction :type "InputAction Object Reference" :default "/Game/Input/Actions/IA_MoveAction.IA_MoveAction"))
  (bind (_x _y) (`KismetMathLibrary.BreakVector2D` ActionValue))
  (:`Triggered`
    (`self.AddMovementInput` (`KismetMathLibrary.Normal` (`KismetMathLibrary.MakeVector` _x (* _y -1.0))) (`self.MoveSpeed`) :!label _label)
    (`self.SetFlipBook` ActionValue))
  (:`Canceled`
    (goto _label))
  (:`Completed`
    (goto _label)))

(event `EnhancedInput|/Game/Input/Actions/IA_Interact`
  (params (ActionValue :type Boolean) (ElapsedSeconds :type "Float (double-precision)") (TriggeredSeconds :type "Float (double-precision)") (InputAction :type "InputAction Object Reference" :default "/Game/Input/Actions/IA_Interact.IA_Interact"))
  (:`Triggered`
    (bind _currentinteractable (`self.CurrentInteractable`)
      (:`then`
        (`/Game/Blueprints/Actor/BP_OverworldInteractionActor.OnInteract` _currentinteractable))
      (:`else`))))

(fn `SetFlipBook`
  (params (MovementVector :type "Vector2D Structure"))
  (locals (XVal :type "Float (double-precision)" :default 0.0) (YVal :type "Float (double-precision)" :default 0.0))
  (bind (_x _y) (`KismetMathLibrary.BreakVector2D` MovementVector))
  (set `local.XVal` _x)
  (set `local.YVal` _y)
  (if (`KismetMathLibrary.IsZero2D` MovementVector)
    (`PaperFlipbookComponent.SetFlipbook` (`self.Sprite`) "/Game/Assets/Textures/OverworldCharacter/OverworldWalkForward.OverworldWalkForward")
    (else
      (`|ExecutionSequence`
        (:`then_0`
          (if (and (!= (`local.XVal`) 0.0) (== (`local.YVal`) 0.0))
            (if (> (`local.XVal`) 0.3)
              (`PaperFlipbookComponent.SetFlipbook` (`self.Sprite`) "/Game/Assets/Textures/OverworldCharacter/OverworldWalkRight.OverworldWalkRight")
              (else
                (`PaperFlipbookComponent.SetFlipbook` (`self.Sprite`) "/Game/Assets/Textures/OverworldCharacter/OverworldWalkLeft.OverworldWalkLeft")))))
        (:`then_1`
          (if (!= (`local.YVal`) 0.0)
            (if (> (`local.YVal`) 0.3)
              (`PaperFlipbookComponent.SetFlipbook` (`self.Sprite`) "/Game/Assets/Textures/OverworldCharacter/OverworldWalkBack.OverworldWalkBack")
              (else
                (`PaperFlipbookComponent.SetFlipbook` (`self.Sprite`) "/Game/Assets/Textures/OverworldCharacter/OverworldWalkForward.OverworldWalkForward")))))))))

(fn `SetInteractable`
  (params (Interactable :type "/Game/Blueprints/Actor/BP_OverworldInteractionActor Object Reference"))
  (bind _output_get (set `self.CurrentInteractable` Interactable))
  ;[1 1 1] Check if null (no interactable)
  (if (`KismetSystemLibrary.IsValid` _output_get)
    (`SceneComponent.SetHiddenInGame` (`self.InteractionIndicator`) false false)
    (`GameplayStatics.PlaySound2D` "/Game/Assets/Sounds/UI/MENU_B_Select.MENU_B_Select" 1.0 1.0 0.0 null null)
    (else
      (`SceneComponent.SetHiddenInGame` (`self.InteractionIndicator`) true false)
      (`GameplayStatics.PlaySound2D` "/Game/Assets/Sounds/UI/MENU_B_Back.MENU_B_Back" 1.0 1.0 0.0 null null))))

(fn `UserConstructionScript`)